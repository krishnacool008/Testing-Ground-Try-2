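; AI controller for patrolling guard NPCs that runs the GuardBehavior tree on the PetrolData blackboard.
; AI perception sets the Enemy key when it senses an actor without the "Bots" tag and clears it when sensing fails.
; Tick turns the PetrollingGuardV2 pawn's aim and shoot flags on whenever a focus actor exists.
; A helper function seeds the WayPoint key from the ThirdPersonCharacter pawn's first target point.
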(event `self.ReceiveBeginPlay`
  (bind _blackboardcomponent (`self.UseBlackboard` "/Game/Dynamic/NPC/AI/PetrolData.PetrolData"))
  (set `self.BlackboardComp` _blackboardcomponent)
  (`self.RunBehaviorTree` "/Game/Dynamic/NPC/AI/GuardBehavior.GuardBehavior"))

(event `self.ReceiveTick`
  (params (DeltaSeconds :type "Float (single-precision)"))
  (bind _aspetrolling_guard_v2 (cast `/Game/Dynamic/NPC/Behavior/PetrollingGuardV2` (`self.K2_GetPawn`)))
  (bind _output_get (set `/Game/Dynamic/NPC/Behavior/PetrollingGuardV2.AimingGuardBP` (`KismetSystemLibrary.IsValid` (`self.GetFocusActor`)) _aspetrolling_guard_v2))
  (set `/Game/Dynamic/NPC/Behavior/PetrollingGuardV2.ShootGuardBP` _output_get _aspetrolling_guard_v2))

(event `self.AIPerception.OnTargetPerceptionUpdated`
  (params (Actor :type "Actor Object Reference") (Stimulus :type "AIStimulus Structure"))
  (bind _enemy (`self.Enemy`))
  (bind _blackboardcomp (`self.BlackboardComp`))
  (if (`self.ActorHasTag` Actor "Bots")
    _
    (elif (`.bSuccessfullySensed` (break `AIStimulus` Stimulus))
      (`BlackboardComponent.SetValueAsObject` _blackboardcomp _enemy Actor)
      (else
        (`BlackboardComponent.ClearValue` _blackboardcomp _enemy)))))

(fn `Param Route Points`
  (params (BlackBoard :type "BlackboardComponent Object Reference"))
  (bind _asthird_person_character (cast `/Game/Static/Trash/ThirdPersonCharacter` (`self.K2_GetPawn`)))
  (`BlackboardComponent.SetValueAsObject` BlackBoard "WayPoint" (`|GetArrayItem` (`/Game/Static/Trash/ThirdPersonCharacter.TargetPoints` _asthird_person_character))))

(fn `UserConstructionScript`)